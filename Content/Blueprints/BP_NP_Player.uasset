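; BP_NP_Player is a player Blueprint with a bow that switches between first-person and third-person views on F3.
; BeginPlay caches the player controller and starts on the first-person camera.
; CameraSwapMethod toggles which camera is active and flips owner-only visibility, showing the first-person mesh and bow in first person and the body mesh in third person.
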(event `Key|F3`
  (params (Key :type "Key Structure"))
  (:`Pressed`
    (`self.CameraSwapMethod`)))

(event `self.ReceiveBeginPlay`
  (`|ExecutionSequence`
    (:`then_0`
      (bind _asplayer_controller (cast `PlayerController` (`self.GetController`)))
      (set `self.PlayerController` _asplayer_controller))
    (:`then_1`
      (`ActorComponent.Deactivate` (`self.ThirdPersonCamera`))
      (`ActorComponent.Activate` (`self.FPSCamera`) false))))

(fn `UserConstructionScript`)